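; Overseer pawn that the player moves along its local forward and right axes.
; MoveForward and MoveRight axis inputs apply a fixed-step local offset each frame, scaled by axis value but not by delta time.
; Movement skips collision sweeps and is blocked while the SelectionWheelActive flag is set.
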(event `InputAxis|MoveForward`
  (params (AxisValue :type "Float (single-precision)"))
  ;[1 1 1] Movement
  (if (`self.SelectionWheelActive`)
    _
    (elif (!= AxisValue 0.0)
      (`self.K2_AddActorLocalOffset` (`KismetMathLibrary.MakeVector` (* AxisValue 25.0))))))

(event `InputAxis|MoveRight`
  (params (AxisValue :type "Float (single-precision)"))
  ;[1 1 1] Movement
  (if (`self.SelectionWheelActive`)
    _
    (elif (!= AxisValue 0.0)
      (`self.K2_AddActorLocalOffset` (`KismetMathLibrary.MakeVector` 0.0 (* AxisValue 25.0))))))

(fn `UserConstructionScript`)